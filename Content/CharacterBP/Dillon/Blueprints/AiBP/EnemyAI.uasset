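; Enemy AI actor that carries a health bar widget and removes itself when its health runs out.
; Every tick it casts the widget component's user widget to AI_Health and sets the bar percent from Health on a 0–100 scale.
; The same tick destroys the actor at zero or below, a check reached only if that cast succeeds.
; A separate ShowHealthbar function makes the widget component visible.
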(event EventTick
  (params (DeltaSeconds :type Float%20%28single-precision%29))
  ;[1 1 1] Assigns the health bar value to the ai's current health.
  (bind _asai_health (Utilities|Casting|CastToAI_Health (UserInterface|GetUserWidgetObject (Variables|Default|GetHealthBarWidget))))
  (Progress|SetPercent (Variables|/Game/CharacterBP/Dillon/Blueprints/Widgets/AI_Health.AI_Health_C|GetHealthBar _asai_health) (/ (Variables|Default|GetHealth) 1e+02))
  (if (<= (Variables|Default|GetHealth) 0.0)
    (Actor|DestroyActor)))

(fn ConstructionScript)

(fn ShowHealthbar
  (Rendering|SetVisibility (Variables|Default|GetHealthBarWidget) true false))