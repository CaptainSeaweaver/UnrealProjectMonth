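; Assault rifle pickup that attaches to the player mesh's back socket when a DashCharacter overlaps and collects it.
; Start and stop events control a looping Fire timer that spawns PlayerBullet actors at the Arrow until ammo runs out, then flags reloading.
; A reload event refills ammo and clears the flag.
; Tick shortens the fire interval under the player's attack-speed buff, with no restore here.
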(event Custom|StartFiring
  ;[1 1 1] Start / Stop spawning bullets.
  (Utilities|Time|SetTimerbyFunctionName 0 "Fire" (Variables|Default|GetfireRate) true))

(event Custom|StopFiring
  ;[1 1 1] Start / Stop spawning bullets.
  (Utilities|Time|ClearTimerbyFunctionName 0 "Fire"))

(event Custom|WeaponReloaded
  ;[1 1 1] Reload current ammo with max ammo.
  (Variables|Default|SetcurrentAmmo (Variables|Default|GetmaxAmmo))
  (Variables|Default|SetisReloading false))

(event EventTick
  (params (DeltaSeconds :type Float%20%28single-precision%29))
  ;[1 1 1] Increase fire rate.
  (bind _asdash_character (Utilities|Casting|CastToDashCharacter (Game|GetPlayerCharacter 0)))
  (if (Variables|/Game/CharacterBP/Blueprints/DashCharacter.DashCharacter_C|GetattackSpeedBuff _asdash_character)
    (Variables|Default|SetfireRate 0.15)))

(event Collision|EventActorBeginOverlap
  (params (OtherActor :type Actor%20Object%20Reference))
  ;[1 1 1] Weapon is collected.
  (bind _asdash_character (Utilities|Casting|CastToDashCharacter OtherActor))
  (bind _result (Default|CollectWeapon _asdash_character self))
  (if _result
    (Transformation|AttachComponentToComponent (Variables|/Script/Engine.Character|GetMesh (Game|GetPlayerCharacter 0)) "Weapon_Back" "SnapToTarget" "SnapToTarget" "SnapToTarget" true)))

(fn ConstructionScript
  (Variables|Default|SetcurrentAmmo (Variables|Default|GetmaxAmmo)))

(fn Fire
  (bind _currentammo (Variables|Default|GetcurrentAmmo))
  (if (and (not (Variables|Default|GetisReloading)) (> _currentammo 0))
    (Math|Integer|DecrementInt _currentammo
      (:%20%20
        (Game|SpawnActorfromClass "/Game/CharacterBP/Dillon/Blueprints/PlayerBP/PlayerBullet.PlayerBullet_C" (Transformation|GetSocketTransform (Variables|Default|GetArrow) "None" "RTS_World") "Undefined" 0 0)))
    (else
      (Variables|Default|SetisReloading true))))