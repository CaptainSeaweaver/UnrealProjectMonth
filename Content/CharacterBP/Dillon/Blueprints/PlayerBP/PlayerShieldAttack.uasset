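; Player shield attack projectile that homes in on shooter enemies and chains from one to the next.
; A detection radius queues living E_Shooter_BP enemies it overlaps, and a DoOnce points the projectile movement's homing target at the first one's hit point.
; When the shield mesh overlaps an enemy, it enables ragdoll physics, deals damage and removes that enemy from the queue.
; The shield then retargets the next queued enemy, or destroys itself when none remain.
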(event OnComponentBeginOverlap(ShieldDetectionRadius)
  (params (OverlappedComponent :type Primitive%20Component%20Object%20Reference) (OtherActor :type Actor%20Object%20Reference) (OtherComp :type Primitive%20Component%20Object%20Reference) (OtherBodyIndex :type Integer) (bFromSweep :type Boolean) (SweepResult :type Hit%20Result%20Structure%20%28by%20ref%29))
  (bind _entitiestodamage (Variables|Default|GetEntitiesToDamage))
  ;[1 1 1] Collision event to detect enemies.
  (bind _ase_shooter_bp (Utilities|Casting|CastToE_Shooter_BP OtherActor))
  (if (> (Variables|/Game/EnemiesBP/Thomas/E_Shooter_BP.E_Shooter_BP_C|GetHealth _ase_shooter_bp) 0.0)
    (Utilities|Array|Add _entitiestodamage _ase_shooter_bp)
    ;[1 1 1] Home onto target.
    (Utilities|FlowControl|DoOnce false
      (:Completed
        (bind _ase_shooter_bp_2 (Utilities|Casting|CastToE_Shooter_BP (Utilities|Array|Get(acopy) _entitiestodamage)))
        (Variables|/Script/Engine.ProjectileMovementComponent|SetHomingTargetComponent (Variables|Default|GetProjectileMovement) (Variables|/Game/EnemiesBP/Thomas/E_Shooter_BP.E_Shooter_BP_C|GetPlaceForShieldToHit _ase_shooter_bp_2))))))

(event OnComponentBeginOverlap(ShieldMesh)
  (params (OverlappedComponent :type Primitive%20Component%20Object%20Reference) (OtherActor :type Actor%20Object%20Reference) (OtherComp :type Primitive%20Component%20Object%20Reference) (OtherBodyIndex :type Integer) (bFromSweep :type Boolean) (SweepResult :type Hit%20Result%20Structure%20%28by%20ref%29))
  (bind _entitiestodamage (Variables|Default|GetEntitiesToDamage))
  ;[1 1 1] Collision events with enemy.
  (bind _ase_shooter_bp (Utilities|Casting|CastToE_Shooter_BP OtherActor))
  (Physics|SetSimulatePhysics (Variables|/Script/Engine.Character|GetMesh _ase_shooter_bp) true)
  (Default|TwakeDwamage _ase_shooter_bp 1e+02)
  (Utilities|Array|RemoveItem _entitiestodamage _ase_shooter_bp)
  ;[1 1 1] Target next enemy or destroy the shield.
  (if (>= (Utilities|Array|LastIndex _entitiestodamage) 0)
    (bind _ase_shooter_bp_2 (Utilities|Casting|CastToE_Shooter_BP (Utilities|Array|Get(acopy) _entitiestodamage)))
    (Variables|/Script/Engine.ProjectileMovementComponent|SetHomingTargetComponent (Variables|Default|GetProjectileMovement) (Variables|/Game/EnemiesBP/Thomas/E_Shooter_BP.E_Shooter_BP_C|GetPlaceForShieldToHit _ase_shooter_bp_2))
    (else
      (Actor|DestroyActor))))

(fn ConstructionScript)