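; Player bullet actor that damages enemies it overlaps.
; On overlap it subtracts BulletDamage directly from the Health of EnemyAI or E_Sprinter_BP and destroys itself, ignores PlayerShield and PlayerController, and is destroyed by anything else.
; Every tick it casts the player character to Dash, Shield or AOE types and sets a fixed boosted damage when that character's DamageBuff is active.
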(event EventTick
  (params (DeltaSeconds :type Float%20%28single-precision%29))
  ;[1 1 1] Increase bullet damage.
  (bind _asdash_character (Utilities|Casting|CastToDashCharacter (Game|GetPlayerCharacter 0))
    (:then
      (if (Variables|/Game/CharacterBP/Blueprints/DashCharacter.DashCharacter_C|GetdamageBuff _asdash_character)
        (Variables|Default|SetbulletDamage 2e+01)))
    (:CastFailed
      (bind _asshield_character (Utilities|Casting|CastToShieldCharacter (Game|GetPlayerCharacter 0))
        (:then
          (if (Variables|/Game/CharacterBP/Blueprints/ShieldCharacter.ShieldCharacter_C|GetdamageBuff _asshield_character)
            (Variables|Default|SetbulletDamage 2e+01)))
        (:CastFailed
          (bind _asaoe_character (Utilities|Casting|CastToAOE_Character (Game|GetPlayerCharacter 0)))
          (if (Variables|/Game/CharacterBP/Blueprints/AOE_Character.AOE_Character_C|GetdamageBuff _asaoe_character)
            (Variables|Default|SetbulletDamage 2e+01)))))))

(event Collision|EventActorBeginOverlap
  (params (OtherActor :type Actor%20Object%20Reference))
  ;[1 1 1] If we hit an enemy, destroy the bullet then deal damage, otherwise destroy the bullet.
  (bind _asenemy_ai (Utilities|Casting|CastToEnemyAI OtherActor)
    (:then
      (Actor|DestroyActor)
      (Variables|/Game/CharacterBP/Dillon/Blueprints/AiBP/EnemyAI.EnemyAI_C|SetHealth _asenemy_ai (- (Variables|/Game/CharacterBP/Dillon/Blueprints/AiBP/EnemyAI.EnemyAI_C|GetHealth _asenemy_ai) (Variables|Default|GetbulletDamage))))
    (:CastFailed
      (bind _ase_sprinter_bp (Utilities|Casting|CastToE_Sprinter_BP OtherActor)
        (:then
          (Actor|DestroyActor)
          (Variables|/Game/EnemiesBP/Thomas/E_Sprinter_BP.E_Sprinter_BP_C|SetHealth _ase_sprinter_bp (- (Variables|/Game/EnemiesBP/Thomas/E_Sprinter_BP.E_Sprinter_BP_C|GetHealth _ase_sprinter_bp) (Variables|Default|GetbulletDamage))))
        (:CastFailed
          (Utilities|Casting|CastToPlayerShield OtherActor
            (:CastFailed
              (Utilities|Casting|CastToPlayerController OtherActor
                (:CastFailed
                  (Actor|DestroyActor))))))))))

(fn ConstructionScript)