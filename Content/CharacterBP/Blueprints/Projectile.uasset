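; Projectile actor that damages enemies it overlaps, with its collision sphere set to ignore the instigator when moving.
; A cast chain routes Damage to the matching damage function on RecptBoss (truncated to an integer), E_Shooter_BP or E_Sprinter_BP.
; One second after spawning it destroys its mesh and sphere components but not the actor itself, and hits do not end it early.
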(event EventBeginPlay
  (Collision|IgnoreActorwhenMoving (Variables|Default|GetSphere) (Game|GetInstigator) true)
  (Utilities|FlowControl|Delay 1.0)
  (Components|DestroyComponent (Variables|Default|GetBulletMesh))
  (Components|DestroyComponent (Variables|Default|GetSphere)))

(event Collision|EventActorBeginOverlap
  (params (OtherActor :type Actor%20Object%20Reference))
  (bind _asrecpt_boss (Utilities|Casting|CastToRecptBoss OtherActor)
    (:then
      (Default|TakeDamage _asrecpt_boss (Math|Float|Truncate (Variables|Default|GetDamage))))
    (:CastFailed
      (bind _ase_shooter_bp (Utilities|Casting|CastToE_Shooter_BP OtherActor)
        (:then
          (Default|TwakeDwamage _ase_shooter_bp (Variables|Default|GetDamage)))
        (:CastFailed
          (bind _ase_sprinter_bp (Utilities|Casting|CastToE_Sprinter_BP OtherActor))
          (Default|TakeDamawge _ase_sprinter_bp (Variables|Default|GetDamage)))))))

(fn ConstructionScript)