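; BP_EnemyCounter is a level actor that tallies Shooter, Sprinter and Shielder enemies and prints the total, apparently for debugging.
; On BeginPlay it loops over all actors of each class, storing the last array index as that type's count (one short of the real number), and sums them into NumEnemies.
; Tick prints that unchanging total through a three-second Delay.
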(event EventBeginPlay
  (bind _outactors (Actor|GetAllActorsOfClass "/Game/EnemiesBP/Thomas/Enemies/Shooter/E_Shooter_BP.E_Shooter_BP_C"))
  (for (_ _array_index) _outactors
    (Variables|Default|SetNum_Shooters _array_index))
  (bind _outactors_2 (Actor|GetAllActorsOfClass "/Game/EnemiesBP/Thomas/Enemies/Sprinters/E_Sprinter_BP.E_Sprinter_BP_C"))
  (for (_ _array_index_2) _outactors_2
    (Variables|Default|SetNum_Sprinters _array_index_2))
  (bind _outactors_3 (Actor|GetAllActorsOfClass "/Game/EnemiesBP/Thomas/Enemies/Shielders/E_Shielder_BP.E_Shielder_BP_C"))
  (for (_ _array_index_3) _outactors_3
    (Variables|Default|SetNum_Sheilders _array_index_3))
  (Variables|Default|SetNum_Enemies (+ (Variables|Default|GetNum_Shooters) (Variables|Default|GetNum_Sprinters) (Variables|Default|GetNum_Sheilders))))

(event Collision|EventActorBeginOverlap
  (params (OtherActor :type Actor%20Object%20Reference)))

(event EventTick
  (params (DeltaSeconds :type Float%20%28single-precision%29))
  (Utilities|FlowControl|Delay 3.0)
  (Development|PrintString (Utilities|String|ToString(Integer) (Variables|Default|GetNum_Enemies))))

(fn ConstructionScript)