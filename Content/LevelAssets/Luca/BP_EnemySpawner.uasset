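; Enemy spawner that fills up to seven spawn points with a random mix of Sprinter, Shooter and Shielder enemies on BeginPlay.
; A loop walks an array of actors, spawning one enemy at each transform and advancing a counter.
; Each pass has a one-in-ten chance to stop early, so later points may stay empty.
; Type selection uses two successive random rolls, which favours Shielders over Sprinters and Shooters.
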(event EventBeginPlay
  (bind _returnvalue (Math|Random|RandomIntegerinRange 0 2))
  (bind _array (Utilities|Array|MakeArray 0 0 0 0 0 0 0))
  (while (and (not (== (Variables|Default|GetCounter) (Utilities|Array|Length _array))) (not (== (Math|Random|RandomIntegerinRange 0 9) 5)))
    (if (== _returnvalue 0)
      (Game|SpawnActorfromClass "/Game/EnemiesBP/Thomas/Enemies/Sprinters/E_Sprinter_BP.E_Sprinter_BP_C" (Transformation|GetActorTransform (Utilities|Array|Get(acopy) _array (Variables|Default|GetCounter))) "Undefined" 0 0)
      (bind _result (Math|Integer|IncrementInt (Variables|Default|GetCounter))
        (:%20%20
          (Variables|Default|SetCounter _result)))
      (elif (== _returnvalue 1)
        (Game|SpawnActorfromClass "/Game/EnemiesBP/Thomas/Enemies/Shooter/E_Shooter_BP.E_Shooter_BP_C" (Transformation|GetActorTransform (Utilities|Array|Get(acopy) _array (Variables|Default|GetCounter))) "Undefined" 0 0)
        (bind _result_2 (Math|Integer|IncrementInt (Variables|Default|GetCounter))
          (:%20%20
            (Variables|Default|SetCounter _result_2)))
        (else
          (Game|SpawnActorfromClass "/Game/EnemiesBP/Thomas/Enemies/Sheilders/E_Sheilder_BP.E_Sheilder_BP_C" (Transformation|GetActorTransform (Utilities|Array|Get(acopy) _array (Variables|Default|GetCounter))) "Undefined" 0 0)
          (bind _result_3 (Math|Integer|IncrementInt (Variables|Default|GetCounter))
            (:%20%20
              (Variables|Default|SetCounter _result_3))))))))

(fn ConstructionScript)