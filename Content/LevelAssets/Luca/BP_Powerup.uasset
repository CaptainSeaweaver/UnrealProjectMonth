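; BP_Powerup is a random powerup spawner that creates a buff actor at its own transform on BeginPlay.
; A chain of branches picks between fire rate, damage, see-health, slow-time and speed buffs.
; Each branch makes its own random roll, so earlier buffs are likelier and sometimes nothing spawns.
; The spawner does not destroy itself afterward.
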(event EventBeginPlay
  (bind _returnvalue (Transformation|GetActorTransform))
  (bind _returnvalue_2 (Math|Random|RandomIntegerinRange 0 4))
  (if (== _returnvalue_2 0)
    (Game|SpawnActorfromClass "/Game/CharacterBP/Dillon/Blueprints/PlayerBuffs/FireRateBuff.FireRateBuff_C" _returnvalue "Undefined" 0 0)
    (elif (== _returnvalue_2 1)
      (Game|SpawnActorfromClass "/Game/CharacterBP/Dillon/Blueprints/PlayerBuffs/IncreaseDamageBuff.IncreaseDamageBuff_C" _returnvalue "Undefined" 0 0)
      (elif (== _returnvalue_2 2)
        (Game|SpawnActorfromClass "/Game/CharacterBP/Dillon/Blueprints/PlayerBuffs/SeeHealthBuff.SeeHealthBuff_C" _returnvalue "Undefined" 0 0)
        (elif (== _returnvalue_2 3)
          (Game|SpawnActorfromClass "/Game/CharacterBP/Dillon/Blueprints/PlayerBuffs/SlowTimeBuff.SlowTimeBuff_C" _returnvalue "Undefined" 0 0)
          (elif (== _returnvalue_2 4)
            (Game|SpawnActorfromClass "/Game/CharacterBP/Dillon/Blueprints/PlayerBuffs/SpeedBuff.SpeedBuff_C" _returnvalue "Undefined" 0 0)))))))

(fn ConstructionScript)