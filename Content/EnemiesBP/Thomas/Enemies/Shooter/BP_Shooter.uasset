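; BP_Shooter is an enemy that detects the player by sight and can be damaged and killed.
; When perception updates and the blackboard has no valid Player, it scans sight-perceived actors for a ThirdPersonCharacter and stores it in the Player key.
; TakeDamage subtracts from Health and calls Death at zero or below, which destroys the actor.
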(event OnPerceptionUpdated(AIPerception)
  (params (UpdatedActors :type Array%20of%20Actor%20Object%20References))
  (Utilities|IsValid (AI|Components|Blackboard|GetValueasObject (AI|GetBlackboard 0) (Utilities|Name|MakeLiteralName "Player"))
    (:Is%20Not%20Valid
      (bind _array_element (Utilities|Array|ForEachLoopwithBreak (Class|AIPerceptionComponent|GetCurrentlyPerceivedActors (Variables|Default|GetAIPerception) "/Script/AIModule.AISense_Sight") :!label _label)
        (:LoopBody
          (bind _asthird_person_character (Utilities|Casting|CastToThirdPersonCharacter _array_element))
          (AI|Components|Blackboard|SetValueasObject (AI|GetBlackboard 0) (Utilities|Name|MakeLiteralName "Player") _asthird_person_character)
          (goto _label Break))))))

(event Custom|Death
  (Actor|DestroyActor))

(fn ConstructionScript)

(fn TakeDamage
  (params (DamageDelt :type Integer))
  (bind _output_get (Variables|Default|SetHealth (- (Variables|Default|GetHealth) DamageDelt)))
  (if (<= _output_get 0)
    (CallFunction|Death)))